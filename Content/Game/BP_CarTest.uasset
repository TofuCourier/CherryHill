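; BP_CarTest is a test car actor that drives along the spline of its Road reference.
; Each tick it advances Distance by Speed, teleports to that spline location and updates the spline.
; It hides its static mesh, without destroying the actor, within 50 units of spline point 1.
; The disconnected lookup of BP_SplineTest roads is noted as moved to a traffic manager.
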(event `self.ReceiveTick`
  (params (DeltaSeconds :type "Float (single-precision)"))
  (bind _spline (`/Game/Game/BP_SplineTest.Spline` (`self.Road`)))
  (bind _returnvalue_location (`KismetMathLibrary.BreakTransform` (`SplineComponent.GetTransformAtSplinePoint` _spline 1 "World" false)))
  (bind _output_get (set `self.Distance` (+ (* DeltaSeconds (`self.Speed`)) (`self.Distance`))))
  (bind _returnvalue (`SplineComponent.GetLocationAtDistanceAlongSpline` _spline _output_get "World"))
  (`self.K2_SetActorLocation` _returnvalue false true)
  (`SplineComponent.UpdateSpline` _spline)
  (if (== _returnvalue _returnvalue_location :`ErrorTolerance` 50.0)
    (`SceneComponent.SetVisibility` (`self.StaticMesh`) false false)))

(fn `UserConstructionScript`)