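; BP_Action_Fly_Up is an action-system action, named for an upward flight move, that currently adds no live behavior of its own.
; Its Initialize, StartAction and StopAction events only call the parent implementations.
; Disconnected nodes hold an unfinished or abandoned boost that casts the instigator to the first-person character and launches it vertically at a speed interpolated toward MaxSpeed.
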(event `self.Initialize`
  (params (Instigator :type "Actor Object Reference"))
  (`parent.Initialize` Instigator))

(event `self.StartAction`
  (params (Instigator :type "Actor Object Reference"))
  (`parent.StartAction` Instigator))

(event `self.StopAction`
  (params (Instigator :type "Actor Object Reference"))
  (`parent.StopAction` Instigator))