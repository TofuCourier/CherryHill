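; BP_TrafficManager spawns traffic cars onto the level's spline roads.
; On BeginPlay it collects every BP_SplineTest actor into Roads and starts a looping timer that calls SpawnCar.
; Each call spawns a new, unpooled BP_CarTest at a road's transform and sets its Road reference.
; Transform and reference come from separate RandomStream picks, so they can point to different roads.
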(event `self.ReceiveBeginPlay`
  ; Construction?
  (bind _outactors (`GameplayStatics.GetAllActorsOfClass` "/Game/Game/BP_SplineTest.BP_SplineTest_C"))
  (for _array_element _outactors
    (`KismetArrayLibrary.Array_Add` (`self.Roads`) _array_element))
  (`KismetSystemLibrary.K2_SetTimerDelegate` (delegate `SpawnCar`) 0.5 true))

(event `SpawnCar`
  (bind _outitem (`KismetArrayLibrary.Array_RandomFromStream` (`self.Roads`) (`self.Random Stream`)))
  ; Should pool this
  (bind _returnvalue (`|SpawnActorFromClass` "/Game/Game/BP_CarTest.BP_CarTest_C" (`self.GetTransform` _outitem) "Undefined" "MultiplyWithRoot" self null))
  (set `/Game/Game/BP_CarTest.Road` _outitem _returnvalue))

(fn `UserConstructionScript`)