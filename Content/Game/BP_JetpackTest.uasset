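; BP_JetpackTest is a test jetpack Blueprint that attaches itself to the Character who interacts with it.
; Interact casts the instigator to Character and calls AttachJetpack, printing an error if the cast fails, while GetInteractText returns an empty string.
; Tick is empty, with a TODO about boost decay.
; Disconnected nodes would spawn the MS_Jetpack sound and feed BoostCharge into its Boost parameter, but never run.
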(event `self.ReceiveBeginPlay`)

(event `CHGameplayInterface.Interact`
  (params (InstigatorPawn :type "Pawn Object Reference"))
  (bind _ascharacter (cast `Character` InstigatorPawn)
    (:`then`
      (`self.AttachJetpack` _ascharacter))
    (:`CastFailed`
      (`KismetSystemLibrary.PrintString` "Failed to attach jetpack to character in BP_Jetpacktest"))))

(event `self.ReceiveTick`
  (params (DeltaSeconds :type "Float (single-precision)"))
  ;[0.5156 0.009117 0 0.5] decay work off of the boost? @TODO Move this to c++. Also needs to be switched off
)

(fn `GetInteractText`
  (params (InstigatorPawn :type "Pawn Object Reference"))
  (returns (ReturnValue :type Text))
  (return ""))

(fn `UserConstructionScript`)