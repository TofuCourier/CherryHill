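; Test actor for procedural delivery generation that scatters mail targets across the four side faces of its SpawnableArea box at BeginPlay.
; Each face gets a padded row-by-column grid using target class-default extents, with weighted random rolls placing outward-offset BP_TargetTest actors.
; Only the +X face fills failed rolls with BP_TargetTestDud.
; Spawned targets are initialized with this actor and counted for a debug print; a mail-delivered event increments the delivered count.
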(event `self.ReceiveBeginPlay`
  (bind _boxextents (defaults `/Game/Game/BP_TargetTest` "/Game/Game/BP_TargetTest.BP_TargetTest_C"))
  (bind _boxextents_2 (defaults `/Game/Game/BP_TargetTest` "/Game/Game/BP_TargetTest.BP_TargetTest_C"))
  (bind _boxextents_3 (defaults `/Game/Game/BP_TargetTest` "/Game/Game/BP_TargetTest.BP_TargetTest_C"))
  (bind _boxextents_4 (defaults `/Game/Game/BP_TargetTest` "/Game/Game/BP_TargetTest.BP_TargetTest_C"))
  (bind (_spawnboundsextent_x _spawnboundsextent_y _spawnboundsextent_z) (`KismetMathLibrary.BreakVector` (`self.SpawnBoundsExtent`)))
  (bind _spawnboundsextent_x_2 (`KismetMathLibrary.BreakVector` (`self.SpawnBoundsExtent`)))
  (bind (_spawnboundsextent_x_3 _spawnboundsextent_y_2) (`KismetMathLibrary.BreakVector` (`self.SpawnBoundsExtent`)))
  (bind (_padding_x _padding_y) (`KismetMathLibrary.BreakVector` (`self.Padding`)))
  (bind (_spawnboundsextent_x_4 _spawnboundsextent_y_3 _spawnboundsextent_z_2) (`KismetMathLibrary.BreakVector` (`self.SpawnBoundsExtent`)))
  (bind (_padding_x_2 _padding_y_2) (`KismetMathLibrary.BreakVector` (`self.Padding`)))
  (bind (_padding_x_3 _padding_y_3) (`KismetMathLibrary.BreakVector` (`self.Padding`)))
  (bind (_spawnboundsextent_x_5 _spawnboundsextent_y_4) (`KismetMathLibrary.BreakVector` (`self.SpawnBoundsExtent`)))
  (bind _spawnboundsextent_x_6 (`KismetMathLibrary.BreakVector` (`self.SpawnBoundsExtent`)))
  (bind (_spawnboundsextent_x_7 _spawnboundsextent_y_5) (`KismetMathLibrary.BreakVector` (`self.SpawnBoundsExtent`)))
  (bind (_spawnboundsextent_x_8 _spawnboundsextent_y_6 _spawnboundsextent_z_3) (`KismetMathLibrary.BreakVector` (`self.SpawnBoundsExtent`)))
  (bind _spawnboundsextent_x_9 (`KismetMathLibrary.BreakVector` (`self.SpawnBoundsExtent`)))
  (bind (_spawnboundsextent_x_10 _spawnboundsextent_y_7 _spawnboundsextent_z_4) (`KismetMathLibrary.BreakVector` (`self.SpawnBoundsExtent`)))
  (bind _spawnboundsextent_x_11 (`KismetMathLibrary.BreakVector` (`self.SpawnBoundsExtent`)))
  (bind (_spawnboundsextent_x_12 _spawnboundsextent_y_8) (`KismetMathLibrary.BreakVector` (`self.SpawnBoundsExtent`)))
  (bind (_padding_x_4 _padding_y_4) (`KismetMathLibrary.BreakVector` (`self.Padding`)))
  (bind _returnvalue (- (`self.Num Rows`) 1))
  (bind _returnvalue_2 (- (`self.Num Columns`) 1))
  (bind _returnvalue_3 (- (`self.Num Rows`) 1))
  (bind _returnvalue_4 (- (`self.Num Rows`) 1))
  (bind _returnvalue_5 (- (`self.Num Columns`) 1))
  (bind _returnvalue_6 (- (`self.Num Columns`) 1))
  (bind _returnvalue_7 (- (`self.Num Rows`) 1))
  (bind _returnvalue_8 (- (`self.Num Columns`) 1))
  ; +X   Right(Face) Side
  ;; Set our spawnable origin point
  (set `self.SpawnAreaOrigin` (+ (`self.K2_GetActorLocation`) (`SceneComponent.RelativeLocation` (`self.SpawnableArea`))))
  (set `self.SpawnBoundsExtent` (+ (`BoxComponent.BoxExtent` (`self.SpawnableArea`)) (`KismetMathLibrary.MakeVector` (.z _boxextents) (+ (* (.x _boxextents) -1.0) _padding_x_3) (+ _padding_y_3 (* (.y _boxextents) -1.0)))))
  (for _index (range (+ _returnvalue 1))
    (bind _output_get (set `self.Z` (`KismetMathLibrary.Lerp` (* _spawnboundsextent_z_2 -1.0) _spawnboundsextent_z_2 (/ (`KismetMathLibrary.Conv_IntToDouble` _index) (`KismetMathLibrary.Conv_IntToDouble` _returnvalue)))))
    (for _index_2 (range (+ _returnvalue_2 1))
      (bind _output_get_2 (set `self.Y` (`KismetMathLibrary.Lerp` (* _spawnboundsextent_y_4 -1.0) _spawnboundsextent_y_4 (/ (`KismetMathLibrary.Conv_IntToDouble` _index_2) (`KismetMathLibrary.Conv_IntToDouble` _returnvalue_2)))))
      (bind _output_get_3 (set `self.LocalOffset` (`KismetMathLibrary.MakeVector` 0.0 _output_get_2 _output_get)))
      (if (`KismetMathLibrary.RandomBoolWithWeight` 0.2)
        (bind _returnvalue_9 (+ _output_get_3 (`KismetMathLibrary.MakeVector` _spawnboundsextent_x_9) (`self.SpawnAreaOrigin`)))
        (bind _returnvalue_10 (`|SpawnActorFromClass` "/Game/Game/BP_TargetTest.BP_TargetTest_C" (`KismetMathLibrary.MakeTransform` _returnvalue_9 (struct :`Pitch` -90.0)) "Undefined" "MultiplyWithRoot" null null))
        (`/Game/Game/BP_TargetTest.Initialize` _returnvalue_10 self)
        (`/Engine/EditorBlueprintResources/StandardMacros.IncrementInt` (`self.SpawnedMailboxCount`) :!label _label)
        (else
          (`|SpawnActorFromClass` "/Game/Game/BP_TargetTestDud.BP_TargetTestDud_C" (`KismetMathLibrary.MakeTransform` _returnvalue_9 (struct :`Pitch` -90.0)) "Undefined" "MultiplyWithRoot" null null)))))
  ; -X   Left(Face) Side
  (set `self.SpawnAreaOrigin` (+ (`self.K2_GetActorLocation`) (`SceneComponent.RelativeLocation` (`self.SpawnableArea`))))
  (set `self.SpawnBoundsExtent` (+ (`BoxComponent.BoxExtent` (`self.SpawnableArea`)) (`KismetMathLibrary.MakeVector` (.z _boxextents_3) (+ (* (.x _boxextents_3) -1.0) _padding_x_4) (+ _padding_y_4 (* (.y _boxextents_3) -1.0)))))
  (for _index_3 (range (+ _returnvalue_3 1))
    (bind _output_get_4 (set `self.Z` (`KismetMathLibrary.Lerp` (* _spawnboundsextent_z_3 1.0) (* _spawnboundsextent_z_3 -1.0) (/ (`KismetMathLibrary.Conv_IntToDouble` _index_3) (`KismetMathLibrary.Conv_IntToDouble` _returnvalue_3)))))
    (for _index_4 (range (+ _returnvalue_6 1))
      (bind _output_get_5 (set `self.Y` (`KismetMathLibrary.Lerp` (* _spawnboundsextent_y_5 1.0) (* _spawnboundsextent_y_5 -1.0) (/ (`KismetMathLibrary.Conv_IntToDouble` _index_4) (`KismetMathLibrary.Conv_IntToDouble` _returnvalue_6)))))
      (bind _output_get_6 (set `self.LocalOffset` (`KismetMathLibrary.MakeVector` 0.0 _output_get_5 _output_get_4)))
      (if (`KismetMathLibrary.RandomBoolWithWeight` 0.2)
        (bind _returnvalue_11 (`|SpawnActorFromClass` "/Game/Game/BP_TargetTest.BP_TargetTest_C" (`KismetMathLibrary.MakeTransform` (+ _output_get_6 (`KismetMathLibrary.MakeVector` (* _spawnboundsextent_x_6 -1.0)) (`self.SpawnAreaOrigin`)) (struct :`Pitch` 90.0)) "Undefined" "MultiplyWithRoot" null null))
        (`/Game/Game/BP_TargetTest.Initialize` _returnvalue_11 self)
        (goto _label))))
  ; +Y  Front(Face) Side
  (set `self.SpawnAreaOrigin` (+ (`self.K2_GetActorLocation`) (`SceneComponent.RelativeLocation` (`self.SpawnableArea`))))
  (set `self.SpawnBoundsExtent` (+ (`BoxComponent.BoxExtent` (`self.SpawnableArea`)) (`KismetMathLibrary.MakeVector` (+ (* (.x _boxextents_2) -1.0) _padding_x_2) (.z _boxextents_2) (+ _padding_y_2 (* (.y _boxextents_2) -1.0)))))
  (for _index_5 (range (+ _returnvalue_4 1))
    (bind _output_get_7 (set `self.Z` (`KismetMathLibrary.Lerp` (* _spawnboundsextent_z -1.0) _spawnboundsextent_z (/ (`KismetMathLibrary.Conv_IntToDouble` _index_5) (`KismetMathLibrary.Conv_IntToDouble` _returnvalue_4)))))
    (for _index_6 (range (+ _returnvalue_5 1))
      (bind _output_get_8 (set `self.X` (`KismetMathLibrary.Lerp` (* _spawnboundsextent_x_2 -1.0) _spawnboundsextent_x_2 (/ (`KismetMathLibrary.Conv_IntToDouble` _index_6) (`KismetMathLibrary.Conv_IntToDouble` _returnvalue_5)))))
      (bind _output_get_9 (set `self.LocalOffset` (`KismetMathLibrary.MakeVector` _output_get_8 0.0 _output_get_7)))
      (if (`KismetMathLibrary.RandomBoolWithWeight` 0.2)
        (bind _returnvalue_12 (`|SpawnActorFromClass` "/Game/Game/BP_TargetTest.BP_TargetTest_C" (`KismetMathLibrary.MakeTransform` (+ _output_get_9 (`KismetMathLibrary.MakeVector` 0.0 _spawnboundsextent_y_2) (`self.SpawnAreaOrigin`)) (struct :`Roll` 90.0)) "Undefined" "MultiplyWithRoot" null null))
        (`/Game/Game/BP_TargetTest.Initialize` _returnvalue_12 self)
        (goto _label))))
  ; -Y Rear (Face) Side
  (set `self.SpawnAreaOrigin` (+ (`self.K2_GetActorLocation`) (`SceneComponent.RelativeLocation` (`self.SpawnableArea`))))
  (set `self.SpawnBoundsExtent` (+ (`BoxComponent.BoxExtent` (`self.SpawnableArea`)) (`KismetMathLibrary.MakeVector` (+ (* (.x _boxextents_4) -1.0) _padding_x) (.z _boxextents_4) (+ _padding_y (* (.y _boxextents_4) -1.0)))))
  (for _index_7 (range (+ _returnvalue_7 1))
    (bind _output_get_10 (set `self.Z` (`KismetMathLibrary.Lerp` (* _spawnboundsextent_z_4 -1.0) _spawnboundsextent_z_4 (/ (`KismetMathLibrary.Conv_IntToDouble` _index_7) (`KismetMathLibrary.Conv_IntToDouble` _returnvalue_7)))))
    (for _index_8 (range (+ _returnvalue_8 1))
      (bind _output_get_11 (set `self.X` (`KismetMathLibrary.Lerp` (* _spawnboundsextent_x_11 -1.0) _spawnboundsextent_x_11 (/ (`KismetMathLibrary.Conv_IntToDouble` _index_8) (`KismetMathLibrary.Conv_IntToDouble` _returnvalue_8)))))
      (bind _output_get_12 (set `self.LocalOffset` (`KismetMathLibrary.MakeVector` _output_get_11 0.0 _output_get_10)))
      (if (`KismetMathLibrary.RandomBoolWithWeight` 0.2)
        (bind _returnvalue_13 (`|SpawnActorFromClass` "/Game/Game/BP_TargetTest.BP_TargetTest_C" (`KismetMathLibrary.MakeTransform` (+ _output_get_12 (`KismetMathLibrary.MakeVector` 0.0 (* _spawnboundsextent_y_8 -1.0)) (`self.SpawnAreaOrigin`)) (struct :`Roll` -90.0)) "Undefined" "MultiplyWithRoot" null null))
        (`/Game/Game/BP_TargetTest.Initialize` _returnvalue_13 self)
        (goto _label))))
  (`KismetSystemLibrary.PrintString` (`KismetStringLibrary.Concat_StrStr` "Total Windows : " (`KismetStringLibrary.Conv_IntToString` (`self.SpawnedMailboxCount`))) true true (struct :`R` 0.510417 :`B` 0.018423 :`A` 1.0))
  (add `self.OnMailDelivered` (delegate `OnMailDelivered_Event`)))

(event `OnMailDelivered_Event`
  ; Mail Delivered
  (`/Engine/EditorBlueprintResources/StandardMacros.IncrementInt` (`self.DeliveredMailCount`)))

(fn `SetupStartingCornerPoint`)

(fn `UserConstructionScript`)